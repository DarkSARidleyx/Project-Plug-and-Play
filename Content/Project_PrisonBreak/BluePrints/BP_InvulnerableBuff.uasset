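; BP_InvulnerableBuff is a pickup that grants the player temporary invulnerability.
; It caches the Bp_Player reference on BeginPlay and reacts when an actor tagged Player overlaps its trigger box.
; On pickup it sets InvulnerableBuffActive, moves its sphere below the world and hides itself.
; After a short delay it clears the flag and destroys itself, so the pickup actor itself times the buff.
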(event OnComponentBeginOverlap(triggerBox)
  (params (OverlappedComponent :type Primitive%20Component%20Object%20Reference) (OtherActor :type Actor%20Object%20Reference) (OtherComp :type Primitive%20Component%20Object%20Reference) (OtherBodyIndex :type Integer) (bFromSweep :type Boolean) (SweepResult :type Hit%20Result%20Structure%20%28by%20ref%29))
  (if (Actor|ActorHasTag OtherActor "Player")
    (Development|PrintString "Invulnerable Buff Collected")
    (Variables|/Game/Project_PrisonBreak/BluePrints/Bp_Player.Bp_Player_C|SetInvulnerableBuffActive? (Variables|Default|GetBp%20PlayerRef) true)
    (Transformation|SetWorldLocation (Variables|Default|GetSphere) "0.000000,0.000000,-100.000000" false true)
    (Rendering|SetActorHiddenInGame true)
    (Utilities|FlowControl|Delay 5.0)
    (Development|PrintString "Invulnerable Buff Deactivated")
    (Variables|/Game/Project_PrisonBreak/BluePrints/Bp_Player.Bp_Player_C|SetInvulnerableBuffActive? (Variables|Default|GetBp%20PlayerRef) false)
    (Actor|DestroyActor)))

(event EventBeginPlay
  (bind _asbp_player (Utilities|Casting|CastToBp_Player (Game|GetPlayerCharacter 0)))
  (Variables|Default|SetBp%20PlayerRef _asbp_player))

(fn ConstructionScript)