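; BP_AttackBuff is a rotating syringe pickup that temporarily gives the player an attack buff.
; On BeginPlay it adds a rotating movement component and caches a reference to the player character.
; When a Player-tagged actor overlaps TriggerBox, it sets AttackBuffActive on the player, moves the syringe away and hides itself.
; After a five-second delay it clears the flag and destroys itself, so the pickup actor itself times the buff.
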(event OnComponentBeginOverlap(TriggerBox)
  (params (OverlappedComponent :type Primitive%20Component%20Object%20Reference) (OtherActor :type Actor%20Object%20Reference) (OtherComp :type Primitive%20Component%20Object%20Reference) (OtherBodyIndex :type Integer) (bFromSweep :type Boolean) (SweepResult :type Hit%20Result%20Structure%20%28by%20ref%29))
  (if (Actor|ActorHasTag OtherActor "Player")
    (Development|PrintString "Attack Buff Collected")
    (Variables|/Game/Project_PrisonBreak/BluePrints/Bp_Player.Bp_Player_C|SetAttackBuffActive? (Variables|Default|GetAs%20Bp%20Player) true)
    (Transformation|SetWorldLocation (Variables|Default|Getsyringe) "0.000000,0.000000,-100.000000" false true)
    (Rendering|SetActorHiddenInGame true)
    (Utilities|FlowControl|Delay 5.0)
    (Development|PrintString "Attack Buff Deactivated" true true "(R=1.000000,G=0.000000,B=0.023098,A=1.000000)" 0.5)
    (Variables|/Game/Project_PrisonBreak/BluePrints/Bp_Player.Bp_Player_C|SetAttackBuffActive? (Variables|Default|GetAs%20Bp%20Player) false)
    (Actor|DestroyActor)))

(event EventBeginPlay
  (AddComponent|AddRotatingMovementComponent)
  (bind _asbp_player (Utilities|Casting|CastToBp_Player (Game|GetPlayerCharacter 0)))
  (Variables|Default|SetAs%20Bp%20Player _asbp_player))

(fn ConstructionScript)