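; BP_StaminaBuff is a rotating pickup that temporarily grants the player a stamina buff.
; On BeginPlay it adds a rotating movement component and caches the Bp_Player reference.
; When a Player-tagged actor overlaps TriggerBox, it sets the player's buff flag, shortens StaminaDelayTimer, moves the cone below the world origin and hides itself.
; After a fixed delay it clears the flag, sets the timer to a hardcoded longer value and destroys itself.
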(event OnComponentBeginOverlap(triggerBox)
  (params (OverlappedComponent :type Primitive%20Component%20Object%20Reference) (OtherActor :type Actor%20Object%20Reference) (OtherComp :type Primitive%20Component%20Object%20Reference) (OtherBodyIndex :type Integer) (bFromSweep :type Boolean) (SweepResult :type Hit%20Result%20Structure%20%28by%20ref%29))
  (bind _bp_playerref (Variables|Default|GetBp%20PlayerRef))
  (bind _bp_playerref_2 (Variables|Default|GetBp%20PlayerRef))
  (if (Actor|ActorHasTag OtherActor "Player")
    (Development|PrintString "Stamina Buff Collected")
    (Variables|/Game/Project_PrisonBreak/BluePrints/Bp_Player.Bp_Player_C|SetStaminaBuffActive? _bp_playerref true)
    (Variables|/Game/Project_PrisonBreak/BluePrints/Bp_Player.Bp_Player_C|SetStaminaDelayTimer _bp_playerref 1.0)
    (Transformation|SetWorldLocation (Variables|Default|GetCone) "0.000000,0.000000,-100.000000" false true)
    (Rendering|SetActorHiddenInGame true)
    (Utilities|FlowControl|Delay 5.0)
    (Development|PrintString "Stamina Buff Deactivated" true true "(R=1.000000,G=0.000000,B=0.023098,A=1.000000)" 0.5)
    (Variables|/Game/Project_PrisonBreak/BluePrints/Bp_Player.Bp_Player_C|SetStaminaBuffActive? _bp_playerref_2 false)
    (Variables|/Game/Project_PrisonBreak/BluePrints/Bp_Player.Bp_Player_C|SetStaminaDelayTimer _bp_playerref_2 5.0)
    (Actor|DestroyActor)))

(event EventBeginPlay
  (AddComponent|AddRotatingMovementComponent)
  (bind _asbp_player (Utilities|Casting|CastToBp_Player (Game|GetPlayerCharacter 0)))
  (Variables|Default|SetBp%20PlayerRef _asbp_player))

(fn ConstructionScript)