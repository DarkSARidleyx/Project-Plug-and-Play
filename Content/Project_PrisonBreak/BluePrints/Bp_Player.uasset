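; Paper2D player character that runs, jumps, taunts, attacks, toggles a pause menu and quits the game on death.
; Input swaps Sprite flipbooks, with finished animations resetting to idle and clearing attack flags, and jumps polling Z velocity for landing.
; Tick checks for zero health and, while attacking, damages HitBox overlaps every frame by attack type.
; The heavy attack key sets IsHeavyAttack false, so its damage branch never runs.
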(event OnFinishedPlaying(Sprite)
  ;[1 0 0] Resets Sprite After Each Flipbook is finished playing sets it back to idle
  (Sprite|SetFlipbook (Variables|Default|GetSprite) "/Game/Project_PrisonBreak/Character_Sprites/GuywithBat/Raider_3/Flipbooks/FP_Idle1.FP_Idle1")
  (CallFunction|RestartAnim)
  (Variables|Default|SetisAttacking? false)
  (Variables|Default|SetisLightAttack? false)
  (Variables|Default|SetisRegularAttack? false)
  (Variables|Default|SetisHeavyAttack? false))

(event Custom|DeathAnimCheck
  ;[1 0 0] Plays Death Anim When Health is Zero
  (if (== (Variables|Default|GetHealth) 0.0)
    (Development|PrintString "Died" true false)
    (Sprite|SetFlipbook (Variables|Default|GetSprite) "/Game/Project_PrisonBreak/Character_Sprites/GuywithBat/Raider_3/Flipbooks/FP_Dead.FP_Dead")
    (Components|Timeline|SetLooping (Variables|Default|GetSprite) false)
    (Utilities|FlowControl|Delay 0.8)
    (Game|QuitGame 0 "Quit" false)))

(event Input|EnhancedActionEvents|EnhancedInputActionIA_Jump
  (params (ActionValue :type Boolean) (ElapsedSeconds :type Float%20%28double-precision%29) (TriggeredSeconds :type Float%20%28double-precision%29) (InputAction :type Input%20Action%20Object%20Reference :default "/Game/Project_PrisonBreak/BluePrints/IA_Jump.IA_Jump"))
  (bind _sprite (Variables|Default|GetSprite))
  ;[1 1 1] Basic Movement
  (if (not (Variables|Default|GetBIsJumping))
    (Variables|Default|SetBIsJumping true)
    (Character|Jump)
    (Components|Timeline|SetLooping _sprite false)
    (Sprite|SetFlipbook _sprite "/Game/Project_PrisonBreak/Character_Sprites/GuywithBat/Raider_3/Flipbooks/FP_Jump.FP_Jump")
    (Utilities|FlowControl|Delay 0.01)
    (if (== (.Z (Math|Vector|BreakVector (Transformation|GetVelocity))) 0.0) :!label _label
      (Components|Timeline|SetLooping _sprite true)
      (Audio|Components|Audio|Play _sprite)
      (Sprite|SetFlipbook _sprite "/Game/Project_PrisonBreak/Character_Sprites/GuywithBat/Raider_3/Flipbooks/FP_Idle1.FP_Idle1")
      (Variables|Default|SetBIsJumping false)
      (else
        (Utilities|FlowControl|Delay 0.01)
        (goto _label)))))

(event Input|EnhancedActionEvents|EnhancedInputActionIA_Movement
  (params (ActionValue :type Float%20%28double-precision%29) (ElapsedSeconds :type Float%20%28double-precision%29) (TriggeredSeconds :type Float%20%28double-precision%29) (InputAction :type Input%20Action%20Object%20Reference :default "/Game/Project_PrisonBreak/BluePrints/IA_Movement.IA_Movement"))
  ;[1 1 1] Basic Movement
  (:Triggered
    (if (not (Variables|Default|GetBIsJumping))
      (Pawn|Input|AddMovementInput (Transformation|GetActorForwardVector) ActionValue false)
      (Sprite|SetFlipbook (Variables|Default|GetSprite) "/Game/Project_PrisonBreak/Character_Sprites/GuywithBat/Raider_3/Flipbooks/FP_Run.FP_Run")
      (if (> ActionValue 0.0)
        (Transformation|SetWorldRotation (Variables|Default|GetSprite) "0, 0, 0" false false)
        (else
          (Transformation|SetWorldRotation (Variables|Default|GetSprite) "0.000000,180.000000,0.000000" false false)))))
  (:Completed
    (if (not (Variables|Default|GetBIsJumping))
      (Sprite|SetFlipbook (Variables|Default|GetSprite) "/Game/Project_PrisonBreak/Character_Sprites/GuywithBat/Raider_3/Flipbooks/FP_Idle1.FP_Idle1"))))

(event EventBeginPlay
  (bind _returnvalue (Game|GetPlayerController 0))
  (bind _asbp_controller (Utilities|Casting|CastToBp_controller (Pawn|GetController)))
  (Input|AddMappingContext (PlayerController|LocalPlayerSubsystems|GetEnhancedInputLocalPlayerSubsystem _asbp_controller) "/Game/Project_PrisonBreak/BluePrints/IMC_Default.IMC_Default" 0 "(bIgnoreAllPressedKeysUntilRelease=True,bForceImmediately=False,bNotifyUserSettings=False)")
  (Input|SetInputModeGameOnly _returnvalue false)
  (Variables|/Script/Engine.PlayerController|SetbShowMouseCursor _returnvalue false))

(event EventTick
  (params (DeltaSeconds :type Float%20%28single-precision%29))
  (CallFunction|DeathAnimCheck)
  (if (Variables|Default|GetisAttacking?)
    (CallFunction|HitCheck)))

(event Game|Damage|EventAnyDamage
  (params (Damage :type Float%20%28single-precision%29) (DamageType :type Damage%20Type%20Object%20Reference) (InstigatedBy :type Controller%20Object%20Reference) (DamageCauser :type Actor%20Object%20Reference))
  ;[1 0 0] Applys Dmg to player Health and triggers the hurt Flipbook per each damage collision
  (Variables|Default|SetHealth (- (Variables|Default|GetHealth) Damage))
  (Sprite|SetFlipbook (Variables|Default|GetSprite) "/Game/Project_PrisonBreak/Character_Sprites/GuywithBat/Raider_3/Flipbooks/FP_Hurt.FP_Hurt")
  (Components|Timeline|SetLooping (Variables|Default|GetSprite) false))

(event Input|KeyboardEvents|P
  (params (Key :type Key%20Structure :default "None"))
  (bind _returnvalue (Game|GetPlayerController 0))
  (bind _returnvalue_2 (Game|GetPlayerController 0))
  ;[1 0 0] Pause Menu
  (:Pressed
    (if (not (Variables|Default|GetisPaused?))
      (Variables|Default|SetisPaused? true)
      (bind _returnvalue_3 (UserInterface|CreateWidget "/Game/Project_PrisonBreak/Menus/WBP_PauseMenu.WBP_PauseMenu_C"))
      (bind _output_get (Variables|Default|SetPauseMenuWidget _returnvalue_3))
      (UserInterface|Viewport|AddtoViewport _output_get 0)
      (Input|SetInputModeGameandUI _returnvalue_2 (Variables|Default|GetPauseMenuWidget) "DoNotLock" true false)
      (Variables|/Script/Engine.PlayerController|SetbShowMouseCursor _returnvalue_2 true)
      (Game|SetGamePaused true)
      (else
        (Variables|Default|SetisPaused? false)
        (Widget|RemovefromParent (Variables|Default|GetPauseMenuWidget))
        (Game|SetGamePaused false)
        (Input|SetInputModeGameOnly _returnvalue false)
        (Variables|/Script/Engine.PlayerController|SetbShowMouseCursor _returnvalue false)))))

(event Input|KeyboardEvents|1
  (params (Key :type Key%20Structure :default "None"))
  ;[1 0.6456 0] Dmg Test
  (:Pressed
    (bind _returnvalue (Game|Damage|ApplyDamage self 1e+01 0 0))
    (Variables|Default|SetHealth (- (Variables|Default|GetHealth) _returnvalue))))

(event Input|KeyboardEvents|Q
  (params (Key :type Key%20Structure :default "None"))
  ;[1 0 0] Taunt Setup
  (:Pressed
    (Sprite|SetFlipbook (Variables|Default|GetSprite) "/Game/Project_PrisonBreak/Character_Sprites/GuywithBat/Raider_3/Flipbooks/FP_Taunt.FP_Taunt")
    (Utilities|FlowControl|Delay 1.0)
    (Components|Timeline|SetLooping (Variables|Default|GetSprite) false)))

(event Input|KeyboardEvents|J
  (params (Key :type Key%20Structure :default "None"))
  ;[1 0 0] Attack Setup
  ;;[0.7304 0 1] Light Attack
  (:Pressed
    (Sprite|SetFlipbook (Variables|Default|GetSprite) "/Game/Project_PrisonBreak/Character_Sprites/GuywithBat/Raider_3/Flipbooks/FP_Attack1.FP_Attack1")
    (Components|Timeline|SetLooping (Variables|Default|GetSprite) false)
    (Variables|Default|SetisAttacking? true)
    (Variables|Default|SetisLightAttack? true)
    (Development|PrintString "Light Attack" true true "(R=0.966819,G=1.000000,B=0.000000,A=1.000000)")))

(event Input|KeyboardEvents|K
  (params (Key :type Key%20Structure :default "None"))
  ;[1 0 0] Attack Setup
  ;;[0.6959 0 0.9911] Regular Attack
  (:Pressed
    (Sprite|SetFlipbook (Variables|Default|GetSprite) "/Game/Project_PrisonBreak/Character_Sprites/GuywithBat/Raider_3/Flipbooks/FP_Attack2.FP_Attack2")
    (Components|Timeline|SetLooping (Variables|Default|GetSprite) false)
    (Variables|Default|SetisAttacking? true)
    (Variables|Default|SetisRegularAttack? true)
    (Development|PrintString "Regular Attack" true true "(R=0.083560,G=1.000000,B=0.000000,A=1.000000)")))

(event Input|KeyboardEvents|L
  (params (Key :type Key%20Structure :default "None"))
  ;[1 0 0] Attack Setup
  ;;[0.8404 0 1] Heavy Attack
  (:Pressed
    (Sprite|SetFlipbook (Variables|Default|GetSprite) "/Game/Project_PrisonBreak/Character_Sprites/GuywithBat/Raider_3/Flipbooks/FP_Attack3.FP_Attack3")
    (Components|Timeline|SetLooping (Variables|Default|GetSprite) false)
    (Variables|Default|SetisAttacking? true)
    (Variables|Default|SetisHeavyAttack? false)
    (Development|PrintString "Heavy Attack" true true "(R=0.000000,G=0.878016,B=1.000000,A=1.000000)")))

(fn ConstructionScript)

(fn RestartAnim
  (Components|Timeline|SetLooping (Variables|Default|GetSprite) true)
  (if (not (Audio|Components|Audio|IsPlaying (Variables|Default|GetSprite)))
    (Audio|Components|Audio|Play (Variables|Default|GetSprite))))

(fn HitCheck
  (for _array_element (Collision|GetOverlappingActors (Variables|Default|GetHitBox) 0 :!class /Script/Engine.PrimitiveComponent)
    (if (Variables|Default|GetisLightAttack?)
      (Variables|Default|SetDamageAmu 5.0)
      (bind _returnvalue (Game|Damage|ApplyDamage _array_element (Variables|Default|GetDamageAmu) 0 0 :!label _label))
      (Development|PrintString (Utilities|String|ToString(Float) _returnvalue))
      (elif (Variables|Default|GetisRegularAttack?)
        (Variables|Default|SetDamageAmu 1e+01)
        (goto _label)
        (elif (Variables|Default|GetisHeavyAttack?)
          (Variables|Default|SetDamageAmu 25.0)
          (goto _label))))))