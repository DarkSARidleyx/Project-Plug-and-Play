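; Flying bat enemy that patrols side to side along X from a random starting direction.
; Tick drives movement, and side hits on non-player obstacles reverse it and flip the flipbook sprite, debounced by a DoOnce and delay.
; An attack chain plays a flipbook and damages the player, but nothing shown starts it, and its AIMoveTo logic is unwired.
; EnemyDied extends the parent, setting the death flipbook and destroying the actor immediately.
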(event OnComponentHit(CapsuleComponent)
  (params (HitComponent :type Primitive%20Component%20Object%20Reference) (OtherActor :type Actor%20Object%20Reference) (OtherComp :type Primitive%20Component%20Object%20Reference) (NormalImpulse :type Vector :default "0, 0, 0") (Hit :type Hit%20Result%20Structure%20%28by%20ref%29))
  ;[0.625 0 0] Check for player collision
  (if (!= OtherActor (Game|Player|GetPlayerPawn 0))
    ;[1 0 0] Bat collides with the world collision obstacles delays then automatically changes direction
    (if (!= (.X (Math|Vector|BreakVector (.normal Hit))) 0.0)
      (Utilities|FlowControl|DoOnce false
        (:Completed
          (Variables|Default|SetmoveRight (not (Variables|Default|GetmoveRight)))
          (CallFunction|ToggleFacingDirection)
          (Utilities|FlowControl|Delay 0.75)
          (CallFunction|ResetDirectionChangeCheck))))))

(event Custom|ResetDirectionChangeCheck
  ;[1 0 0] Bat collides with the world collision obstacles delays then automatically changes direction
  (Utilities|FlowControl|DoOnce false) ; enters at Reset
)

(event Custom|Resetting%20AttackTrigger
  ;[1 0 0] Checking for player Collision and triggering the attack player animation
  (Utilities|FlowControl|DoOnce false) ; enters at Reset
)

(event Custom|AttackPlayer
  (bind _as_bp_player (Variables|Default|GetAs%20Bp%20Player))
  ;[1 0 0] Checking for player Collision and triggering the attack player animation
  (Sprite|SetFlipbook (Variables|Default|GetSprite) "/Game/Project_PrisonBreak/Enemy_Characters/Enemy_Sprites/Bat_Sprites/FlipBooks/FB_BatAttack.FB_BatAttack")
  (Components|Timeline|SetLooping (Variables|Default|GetSprite) false)
  (bind _returnvalue (Game|Damage|ApplyDamage (Variables|Default|GetAs%20Bp%20Player) 2.0 0 0))
  (Variables|/Game/Project_PrisonBreak/BluePrints/Bp_Player.Bp_Player_C|SetHealth _as_bp_player (- (Variables|/Game/Project_PrisonBreak/BluePrints/Bp_Player.Bp_Player_C|GetHealth _as_bp_player) _returnvalue))
  (Variables|Default|SetisAttacking? false))

(event EventBeginPlay
  (Variables|Default|SetmoveRight (Math|Random|RandomBool))
  (CallFunction|ToggleFacingDirection)
  (bind _asbp_player (Utilities|Casting|CastToBp_Player (Game|Player|GetPlayerPawn 0)))
  (Variables|Default|SetAs%20Bp%20Player _asbp_player)
  (Variables|Default|SetLevelStartLocation (Transformation|GetWorldLocation (Variables|Default|GetCapsuleComponent))))

(event EventTick
  (params (DeltaSeconds :type Float%20%28single-precision%29))
  (if (not (Variables|Default|GetisAttacking?))
    (Pawn|Input|AddMovementInput "1.000000,0.000000,0.000000" (select (Variables|Default|GetmoveRight) 1.0 -1.0) false)))

(fn ConstructionScript
  (|CallParentFunction))

(fn EnemyDied
  (|CallParentFunction)
  (Sprite|SetFlipbook (Variables|Default|GetSprite) "/Game/Project_PrisonBreak/Enemy_Characters/Enemy_Sprites/Bat_Sprites/FlipBooks/FB_BatDeath.FB_BatDeath")
  (Components|Timeline|SetLooping (Variables|Default|GetSprite) false)
  (Actor|DestroyActor))

(fn ToggleFacingDirection
  (bind _sprite (Variables|Default|GetSprite))
  (bind _returnvalue (Transformation|GetWorldScale _sprite))
  (Transformation|SetWorldScale3D (Variables|Default|GetSprite) (Math|Vector|MakeVector (* (Math|Float|Absolute(Float) (.x _returnvalue)) (select (Variables|Default|GetmoveRight) -1.0 1.0)) (.y _returnvalue) (.z _returnvalue))))