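; BP_EnemyChar is a rat enemy using Paper2D flipbooks for idle, walk, hurt and death, with player-style Enhanced Input movement still wired in.
; AnyDamage lowers Health and plays the hurt flipbook; exactly zero Health triggers death, then quits the game.
; Sphere overlaps flag the player, and Tick compares X positions for direction, but its movement vector is zero.
; HitCheck is empty, and key 1 tests damage.
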(event OnFinishedPlaying(Sprite)
  ;[1 0 0] Resets Sprite After Each Flipbook is finished playing sets it back to idle
  (Sprite|SetFlipbook (Variables|Default|GetSprite) "/Game/Project_PrisonBreak/Enemy_Characters/Rat_Sprites/FB_RatIdle.FB_RatIdle")
  (CallFunction|RestartAnim)
  (Variables|Default|SetisAttacking? false))

(event OnComponentBeginOverlap(Sphere)
  (params (OverlappedComponent :type Primitive%20Component%20Object%20Reference) (OtherActor :type Actor%20Object%20Reference) (OtherComp :type Primitive%20Component%20Object%20Reference) (OtherBodyIndex :type Integer) (bFromSweep :type Boolean) (SweepResult :type Hit%20Result%20Structure%20%28by%20ref%29))
  ;[1 0 0] Checks for Player Char In Range of AI
  (Utilities|Casting|CastToBp_Player OtherActor)
  (Variables|Default|SetisOverlapping? true))

(event OnComponentEndOverlap(Sphere)
  (params (OverlappedComponent :type Primitive%20Component%20Object%20Reference) (OtherActor :type Actor%20Object%20Reference) (OtherComp :type Primitive%20Component%20Object%20Reference) (OtherBodyIndex :type Integer))
  ;[1 0 0] Checks for Player Char In Range of AI
  (Utilities|Casting|CastToBp_Player OtherActor)
  (Variables|Default|SetisOverlapping? false))

(event Custom|DeathAnimCheck
  ;[1 0 0] Plays Death Anim When Health is Zero
  (if (== (Variables|Default|GetHealth) 0.0)
    (Variables|Default|SetisDead? true)))

(event Input|EnhancedActionEvents|EnhancedInputActionIA_Movement
  (params (ActionValue :type Float%20%28double-precision%29) (ElapsedSeconds :type Float%20%28double-precision%29) (TriggeredSeconds :type Float%20%28double-precision%29) (InputAction :type Input%20Action%20Object%20Reference :default "/Game/Project_PrisonBreak/BluePrints/IA_Movement.IA_Movement"))
  ;[1 1 1] Basic Movement
  (:Triggered
    (if (not (Variables|Default|GetBIsJumping))
      (Pawn|Input|AddMovementInput (Transformation|GetActorForwardVector) ActionValue false)
      (Sprite|SetFlipbook (Variables|Default|GetSprite) "/Game/Project_PrisonBreak/Enemy_Characters/Rat_Sprites/FB_RatWalk.FB_RatWalk")
      (if (Variables|Default|GetisMovingRight?)
        (Transformation|SetActorRotation (Math|Rotator|MakeRotator 0.0 0.0 0.0))
        (else
          (Transformation|SetActorRotation (Math|Rotator|MakeRotator 0.0 0.0 0.0))))))
  (:Completed
    (if (not (Variables|Default|GetBIsJumping))
      (Sprite|SetFlipbook (Variables|Default|GetSprite) "/Game/Project_PrisonBreak/Enemy_Characters/Rat_Sprites/FB_RatIdle.FB_RatIdle"))))

(event EventBeginPlay
  (bind _returnvalue (Game|GetPlayerController 0))
  (bind _asbp_controller (Utilities|Casting|CastToBp_controller (Pawn|GetController)))
  (Input|AddMappingContext (PlayerController|LocalPlayerSubsystems|GetEnhancedInputLocalPlayerSubsystem _asbp_controller) "/Game/Project_PrisonBreak/BluePrints/IMC_Default.IMC_Default" 0 "(bIgnoreAllPressedKeysUntilRelease=True,bForceImmediately=False,bNotifyUserSettings=False)")
  (Input|SetInputModeGameOnly _returnvalue false)
  (Variables|/Script/Engine.PlayerController|SetbShowMouseCursor _returnvalue false))

(event EventTick
  (params (DeltaSeconds :type Float%20%28single-precision%29))
  ;[1 0 0] Death / Player Range Check
  (CallFunction|DeathAnimCheck)
  (if (Variables|Default|GetisAttacking?)
    (CallFunction|HitCheck)
    (elif (Variables|Default|GetisDead?)
      (Sprite|SetFlipbook (Variables|Default|GetSprite) "/Game/Project_PrisonBreak/Enemy_Characters/Rat_Sprites/FB_RatDeath.FB_RatDeath")
      (Components|Timeline|SetLooping (Variables|Default|GetSprite) false)
      (Utilities|FlowControl|Delay 0.8)
      (Game|QuitGame 0 "Quit" false)
      (elif (Variables|Default|GetisOverlapping?)
        (bind _asbp_player (Utilities|Casting|CastToBp_Player (Game|GetPlayerCharacter 0)))
        (if (>= (- (.x (Transformation|GetWorldLocation (Variables|/Script/Engine.Character|GetCapsuleComponent _asbp_player))) (.x (Transformation|GetWorldLocation (Variables|Collision|GetCapsuleComponent)))) 0.0)
          (Variables|Default|SetisMovingRight? true)
          (Pawn|Input|AddMovementInput "0, 0, 0" (- (.x (Transformation|GetWorldLocation (Variables|/Script/Engine.Character|GetCapsuleComponent _asbp_player))) (.x (Transformation|GetWorldLocation (Variables|Collision|GetCapsuleComponent)))) false)
          (else
            (Variables|Default|SetisMovingRight? false)))))))

(event Game|Damage|EventAnyDamage
  (params (Damage :type Float%20%28single-precision%29) (DamageType :type Damage%20Type%20Object%20Reference) (InstigatedBy :type Controller%20Object%20Reference) (DamageCauser :type Actor%20Object%20Reference))
  ;[1 0 0] Applys Dmg to player Health and triggers the hurt Flipbook per each damage collision
  (Variables|Default|SetHealth (- (Variables|Default|GetHealth) Damage))
  (Sprite|SetFlipbook (Variables|Default|GetSprite) "/Game/Project_PrisonBreak/Enemy_Characters/Rat_Sprites/FB_HurtRat.FB_HurtRat")
  (Components|Timeline|SetLooping (Variables|Default|GetSprite) false))

(event Input|KeyboardEvents|1
  (params (Key :type Key%20Structure :default "None"))
  ;[1 0.6456 0] Dmg Test
  (:Pressed
    (bind _returnvalue (Game|Damage|ApplyDamage self 1e+01 0 0))
    (Variables|Default|SetHealth (- (Variables|Default|GetHealth) _returnvalue))))

(fn ConstructionScript)

(fn RestartAnim
  (Components|Timeline|SetLooping (Variables|Default|GetSprite) true)
  (if (not (Audio|Components|Audio|IsPlaying (Variables|Default|GetSprite)))
    (Audio|Components|Audio|Play (Variables|Default|GetSprite))))

(fn HitCheck)