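; Bp_Player is a 2D flipbook player character with Enhanced Input movement and jumping.
; Movement input runs along the actor's forward vector, switches run and idle flipbooks, and rotates the sprite to face the travel direction.
; Jumping blocks movement input and polls vertical velocity in a short delay loop until it reaches zero, then restores idle.
; Hotkeys apply self-damage to reduce Health and open the pause menu widget.
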(event Input|EnhancedActionEvents|EnhancedInputActionIA_Jump
  (params (ActionValue :type Boolean) (ElapsedSeconds :type Float%20%28double-precision%29) (TriggeredSeconds :type Float%20%28double-precision%29) (InputAction :type Input%20Action%20Object%20Reference :default "/Game/BluePrints/IA_Jump.IA_Jump"))
  (bind _sprite (Variables|Default|GetSprite))
  (if (not (Variables|Default|GetBIsJumping))
    (Variables|Default|SetBIsJumping true)
    (Character|Jump)
    (Components|Timeline|SetLooping _sprite false)
    (Sprite|SetFlipbook _sprite "/Game/Assets/Fp_CharJump.Fp_CharJump")
    (Utilities|FlowControl|Delay 0.01)
    (if (== (.Z (Math|Vector|BreakVector (Transformation|GetVelocity))) 0.0) :!label _label
      (Components|Timeline|SetLooping _sprite true)
      (Audio|Components|Audio|Play _sprite)
      (Sprite|SetFlipbook _sprite "/Game/Assets/Fp_Idle.Fp_Idle")
      (Variables|Default|SetBIsJumping false)
      (else
        (Utilities|FlowControl|Delay 0.01)
        (goto _label)))))

(event Input|EnhancedActionEvents|EnhancedInputActionIA_Movement
  (params (ActionValue :type Float%20%28double-precision%29) (ElapsedSeconds :type Float%20%28double-precision%29) (TriggeredSeconds :type Float%20%28double-precision%29) (InputAction :type Input%20Action%20Object%20Reference :default "/Game/BluePrints/IA_Movement.IA_Movement"))
  (:Triggered
    (if (not (Variables|Default|GetBIsJumping))
      (Pawn|Input|AddMovementInput (Transformation|GetActorForwardVector) ActionValue false)
      (Sprite|SetFlipbook (Variables|Default|GetSprite) "/Game/Assets/Fp_playerRun.Fp_playerRun")
      (if (> ActionValue 0.0)
        (Transformation|SetWorldRotation (Variables|Default|GetSprite) "0, 0, 0" false false)
        (else
          (Transformation|SetWorldRotation (Variables|Default|GetSprite) "0.000000,180.000000,0.000000" false false)))))
  (:Completed
    (if (not (Variables|Default|GetBIsJumping))
      (Sprite|SetFlipbook (Variables|Default|GetSprite) "/Game/Assets/Fp_Idle.Fp_Idle"))))

(event EventBeginPlay
  (bind _asbp_controller (Utilities|Casting|CastToBp_controller (Pawn|GetController)))
  (Input|AddMappingContext (PlayerController|LocalPlayerSubsystems|GetEnhancedInputLocalPlayerSubsystem _asbp_controller) "/Game/BluePrints/IMC_Default.IMC_Default" 0 "(bIgnoreAllPressedKeysUntilRelease=True,bForceImmediately=False,bNotifyUserSettings=False)"))

(event Input|KeyboardEvents|P
  (params (Key :type Key%20Structure :default "None"))
  ;[1 0 0.04851] Pause Menu
  (:Pressed
    (bind _returnvalue (UserInterface|CreateWidget "/Game/Project_PrisonBreak/Menus/WBP_PauseMenu.WBP_PauseMenu_C"))
    (UserInterface|Viewport|AddtoViewport _returnvalue 0)))

(event Input|KeyboardEvents|1
  (params (Key :type Key%20Structure :default "None"))
  (:Pressed
    (bind _returnvalue (Game|Damage|ApplyDamage self 1e+01 0 0))
    (Variables|Default|SetHealth (- (Variables|Default|GetHealth) _returnvalue))))

(fn ConstructionScript)